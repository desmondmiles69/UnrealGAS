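; Gameplay ability that watches the owner's health and triggers death when it reaches zero or below.
; On activation it starts an async attribute-change listener on the owner's Ability System Component and keeps the task to end it with the ability.
; Each change prints the avatar name and new value for debugging.
; At zero or less, it tries to activate abilities matching the Death tag, allowing remote activation.
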(event `self.K2_ActivateAbility`
  (bind (_asynctaskproxy _attribute _newvalue) (`AttributeChangeTask.ListenForAttributeChange` (`self.GetAbilitySystemComponentFromActorInfo`) (struct :`AttributeName` "Health" :`Attribute` "/Script/UnrealGAS.CustomAttributeSet:Health" :`AttributeOwner` "/Script/CoreUObject.Class'/Script/UnrealGAS.CustomAttributeSet'"))
    (:`then`
      (set `self.AttributeChangeTask` _asynctaskproxy))
    (:`OnAttributeChanged`
      (`self.DebugPrintNewHealth` _newvalue)
      (if (<= _newvalue 0.0)
        (`AbilitySystemComponent.TryActivateAbilitiesByTag` (`self.GetAbilitySystemComponentFromActorInfo`) (`BlueprintGameplayTagLibrary.MakeGameplayTagContainerFromTag` (`BlueprintGameplayTagLibrary.MakeLiteralGameplayTag` (struct :`TagName` "Tags.Abilities.Death"))) true)))))

(event `self.K2_OnEndAbility`
  (params (bWasCancelled :type Boolean))
  (bind _attributechangetask (`self.AttributeChangeTask`)
    (:`then`
      (`AttributeChangeTask.Endtask` _attributechangetask))
    (:`else`)))

(fn `DebugPrintNewHealth`
  (params (InDouble :type "Float (double-precision)"))
  (`KismetSystemLibrary.PrintString` (`KismetStringLibrary.Concat_StrStr` "Listening health change for: " (`KismetSystemLibrary.GetDisplayName` (`self.GetAvatarActorFromActorInfo`)) "Current health: " (`KismetStringLibrary.Conv_DoubleToString` InDouble))))