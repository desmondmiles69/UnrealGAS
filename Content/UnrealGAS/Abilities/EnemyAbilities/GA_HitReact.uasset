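; Enemy Gameplay Ability that plays directional hit reactions.
; On activation it waits for the Enemy HitReact gameplay event and ignores it if the owner has the Dead tag.
; It derives a direction name from the owner's forward and the vector to the event instigator, then plays the hit react montage and jumps to the section of that name.
; The graph never calls EndAbility and includes debug prints.
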(event `self.K2_ActivateAbility`
  (bind (_asynctaskproxy _payload) (`AbilityTask_WaitGameplayEvent.WaitGameplayEvent` (struct :`TagName` "Tags.Events.Enemy.HitReact") null)
    (:`EventReceived`
      (if (not (`GameplayTagAssetInterface.HasMatchingGameplayTag` (`self.GetAbilitySystemComponentFromActorInfo`) (struct :`TagName` "Tags.Status.Dead")))
        (`self.PrintDebugEventRecieved` _payload)
        (`self.CacheHitDirectionVectors` (`.Instigator` (break `GameplayEventData` _payload)))
        (`|ExecutionSequence`
          (:`then_0`
            (bind _output_get (set `self.HitDirectionName` (`CustomBlueprintFunctionLibrary.GetHitDirectionName` (`CustomBlueprintFunctionLibrary.GetHitDirection` (`self.ActorForward`) (`self.ToInstigator`)))))
            (`KismetSystemLibrary.PrintString` (`KismetStringLibrary.Conv_NameToString` _output_get)))
          (:`then_1`
            (`AbilityTask_PlayMontageAndWait.CreatePlayMontageAndWaitProxy` "None" (`self.HitReactMontage`)
              (:`then`
                (`self.MontageJumpToSection` (`self.HitDirectionName`))))))))))

(fn `PrintDebugEventRecieved`
  (params (GameplayEventData :type "GameplayEventData Structure (by ref)"))
  (`self.bDrawDebug`
    (:`then`
      (`KismetSystemLibrary.PrintString` (`KismetStringLibrary.Concat_StrStr` "Hit event recieved from actor: " (`KismetSystemLibrary.GetDisplayName` (`.Instigator` (break `GameplayEventData` GameplayEventData))))))
    (:`else`)))