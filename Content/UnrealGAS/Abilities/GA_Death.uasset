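; Gameplay ability that handles character death and respawn.
; On activation it starts the death montage and applies GE_Death to the owner, then runs RespawnCharacter when the montage completes, is interrupted or is cancelled.
; Respawn removes the effect granting the Dead status tag, then on authority resets the BaseCharacter's attributes and moves the same actor to a player start, before ending the ability.
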(event `self.K2_ActivateAbility`
  (bind _returnvalue (`self.GetAbilitySystemComponentFromActorInfo`))
  (`AbilityTask_PlayMontageAndWait.CreatePlayMontageAndWaitProxy` "None" (`self.DeathMontage`)
    (:`then`
      (`AbilitySystemComponent.BP_ApplyGameplayEffectSpecToSelf` _returnvalue (`AbilitySystemComponent.MakeOutgoingSpec` :`self` _returnvalue :`GameplayEffectClass` "/Game/UnrealGAS/Abilities/GameplayEffects/GE_Death.GE_Death_C")))
    (:`OnCompleted`
      (`self.RespawnCharacter` :!label _label))
    (:`OnInterrupted`
      (goto _label))
    (:`OnCancelled`
      (goto _label))))

(event `RespawnCharacter`
  (`|ExecutionSequence`
    (:`then_0`
      (`self.BP_RemoveGameplayEffectFromOwnerWithGrantedTags` (struct :`GameplayTags` (struct :`(TagName` "Tags.Status.Dead"))) 1))
    (:`then_1`
      (`self.K2_HasAuthority`
        (:`True`
          (`|ExecutionSequence`
            (:`then_0`
              ;[0 0.005058 0.15 0.5] Cache Base Character
              (bind _asbase_character (cast `BaseCharacter` (`self.GetAvatarActorFromActorInfo`)))
              (set `self.BaseCharacter` _asbase_character))
            (:`then_1`
              ;[0 0.005058 0.15 0.5] Reset Attributes
              (bind _basecharacter (`self.BaseCharacter`)
                (:`then`
                  (`BaseCharacter.ResetAttributes` _basecharacter))
                (:`else`)))
            (:`then_2`
              ;[0 0.005058 0.15 0.5] Respawn the Character
              (bind _basecharacter_2 (`self.BaseCharacter`)
                (:`then`
                  (`Actor.K2_SetActorLocation` (`self.BaseCharacter`) (`Actor.K2_GetActorLocation` (`GameModeBase.K2_FindPlayerStart` (`GameplayStatics.GetGameMode`) (`Pawn.GetController` _basecharacter_2) "")) false false))
                (:`else`)))))))
    (:`then_2`
      (`self.K2_EndAbility`))))